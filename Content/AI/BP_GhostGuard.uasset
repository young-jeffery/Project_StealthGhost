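; BP_GhostGuard is an AI guard that attaches a rifle to its hand on BeginPlay and stages social encounters with other guards.
; Interaction zone overlaps check death, alert, blackboard target and investigate location, with cooldowns and a DoOnce limiting repeats.
; A facing dot product and random roll choose between passing by or stopping to talk.
; Talking sets interaction keys on both guards' blackboards, then timed delays clear the flags and cooldowns.
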(event OnComponentBeginOverlap(InteractionZone)
  (params (OverlappedComponent :type Primitive%20Component%20Object%20Reference) (OtherActor :type Actor%20Object%20Reference) (OtherComp :type Primitive%20Component%20Object%20Reference) (OtherBodyIndex :type Integer) (bFromSweep :type Boolean) (SweepResult :type Hit%20Result%20Structure%20%28by%20ref%29))
  (bind _returnvalue (Utilities|Name|MakeLiteralName "IsInteracting?"))
  (bind _self self)
  (bind _returnvalue_2 (AI|GetAIController _self))
  (bind _returnvalue_3 (AI|GetBlackboard _returnvalue_2))
  ;[1 0.6337 0.005251 0.5] Guard Interactions
  (bind _asbp_ghost_guard (Utilities|Casting|CastToBP_GhostGuard OtherActor))
  (if (Variables|/Script/Project_StealthGhost.Project_StealthGhostCharacter|GetbIsDead _asbp_ghost_guard) ; Is the overlapping charcater dead?
    (Development|PrintString "Bro is dead" true true "(R=1.000000,G=0.948966,B=0.990620,A=1.000000)")
    (else
      (bind _asghost_aicontroller (Utilities|Casting|CastToGhostAIController (AI|GetAIController self)))
      (if (Class|GhostAIController|IsAlerted _asghost_aicontroller) ; Is the Guard Alerted
        (Development|PrintString "I am Alerted. Leave me" true true "(R=1.000000,G=0.108926,B=0.000000,A=1.000000)")
        (else
          (Utilities|IsValid _returnvalue_2 ; Is my AI Controller valid or not?
            (:Is%20Valid
              (if (!= OtherActor _self) ; Ignore Self
                (Utilities|IsValid (AI|Components|Blackboard|GetValueasObject _returnvalue_3 (Utilities|Name|MakeLiteralName "TargetActor")) ; Is a Target in the Blackboard?
                  (:Is%20Not%20Valid
                    (if (Utilities|Operators|NotEqual(!=) :A (AI|Components|Blackboard|GetValueasVector _returnvalue_3 (Utilities|Name|MakeLiteralName "InvestigateLocation"))) ; There is no investigate location in the blackboard right?
                      (if (not (Variables|Default|GetInteractionCooldown)) ; Am I on an Interaction Cooldown?
                        (Variables|Default|SetInteractionCooldown true)
                        (bind _asbp_ghost_guard_2 (Utilities|Casting|CastToBP_GhostGuard OtherActor)) ; Contains our Guard B's reference
                        (Variables|BP_GhostGuard_C|SetInteractionCooldown _asbp_ghost_guard_2 true)
                        (Utilities|FlowControl|DoOnce false :!pinned true :!label _label ; Prevents the Interaction from happen multiple times immediately
                          (:Completed
                            (Development|PrintString "Sup G" true true "(R=0.000000,G=0.000000,B=0.968750,A=1.000000)")
                            (if (> (Math|Vector|DotProduct (Transformation|GetActorForwardVector) (Transformation|GetActorForwardVector _asbp_ghost_guard_2)) 0.5)
                              (Development|PrintString "Waking in the same direction")
                              (elif (Math|Random|RandomBool)
                                (Development|PrintString "Passing Wave" true true "(R=1.000000,G=0.000000,B=0.908964,A=1.000000)")
                                (else
                                  (Transformation|SetActorRotation (Math|Rotator|MakeRotator 0.0 0.0 (.yaw (Math|Rotator|FindLookatRotation (Transformation|GetActorLocation self) (Transformation|GetActorLocation OtherActor)))))
                                  ;;[0.7188 0.5227 0.002429 0.5] Logic for Stopping to Talk
                                  ;;;[0.15 0.1091 0.000507 0.5] Guard A's Logic
                                  (bind _asghost_aicontroller_2 (Utilities|Casting|CastToGhostAIController (AI|GetAIController self)))
                                  (bind _output_get (Variables|Default|SetLocalBlackboardA (Variables|/Script/Project_StealthGhost.GhostAIController|GetCachedBlackboard _asghost_aicontroller_2)))
                                  (Utilities|IsValid _output_get
                                    (:Is%20Valid
                                      (AI|Components|Blackboard|SetValueasBool _output_get (Utilities|Name|MakeLiteralName "IsInteracting?") true)
                                      (AI|Components|Blackboard|SetValueasObject _output_get (Utilities|Name|MakeLiteralName "InteractTarget") _asbp_ghost_guard_2)
                                      ;;;[0.15 0.1091 0.000507 0.5] Guard B's Logic
                                      (bind _asghost_aicontroller_3 (Utilities|Casting|CastToGhostAIController (AI|GetAIController _asbp_ghost_guard_2)))
                                      (bind _output_get_2 (Variables|Default|SetLocalBlackboard (Variables|/Script/Project_StealthGhost.GhostAIController|GetCachedBlackboard _asghost_aicontroller_3)))
                                      (Utilities|IsValid _output_get_2
                                        (:Is%20Valid
                                          (AI|Components|Blackboard|SetValueasBool _output_get_2 (Utilities|Name|MakeLiteralName "IsInteracting?") true)
                                          (AI|Components|Blackboard|SetValueasObject _output_get_2 (Utilities|Name|MakeLiteralName "InteractTarget") self))))))))
                            ;;[0.7188 0.5227 0.002429 0.5] Delays before next loop and Resetting of values to avoid break
                            (Utilities|FlowControl|Delay 4.0)
                            ;;;[0.15 0.1091 0.000507 0.5] Reset Guard B's Values
                            (Utilities|IsValid _output_get_2
                              (:Is%20Valid
                                (AI|Components|Blackboard|SetValueasBool _output_get_2 _returnvalue false)
                                ;;;[0.15 0.1091 0.000507 0.5] Reset Guard A's Values
                                (Utilities|IsValid _output_get
                                  (:Is%20Valid
                                    (AI|Components|Blackboard|SetValueasBool _output_get _returnvalue false)
                                    (Utilities|FlowControl|Delay 5.0)
                                    (Variables|BP_GhostGuard_C|SetInteractionCooldown _asbp_ghost_guard_2 false)
                                    (Variables|Default|SetInteractionCooldown false)
                                    (goto _label Reset)))))))))))))))))))

(event EventBeginPlay
  ;[1 0.5409 0 0.5] Spawn Guards Weapon
  (bind _returnvalue (Game|SpawnActorfromClass "/Game/AI/BP_RifleEquipment.BP_RifleEquipment_C" (Math|Transform|MakeTransform "0, 0, 0" "0, 0, 0" "1.000000,1.000000,1.000000") "Undefined" "MultiplyWithRoot" 0 0))
  (Transformation|AttachComponentToComponent _returnvalue (Variables|Character|GetMesh) "enemyshoot_righthand" "SnapToTarget" "SnapToTarget" "KeepRelative" true))

(fn ConstructionScript)